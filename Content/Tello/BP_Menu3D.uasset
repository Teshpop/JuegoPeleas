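; BP_Menu3D is an in-world 3D menu actor that hands the player's view over to linked menus.
; On BeginPlay it binds to the transition event of its WBP_Menu3D widget, which passes an index into the LinkedMenus array.
; A valid index disables collision on this menu, enables it on the target and cubically blends the player camera to that menu actor.
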(event Custom|TransitionTo
  (params (NewParam :type BP%20Menu%203D%20Object%20Reference))
  (Collision|SetActorEnableCollision false)
  (Collision|SetActorEnableCollision NewParam true)
  (Game|Player|SetViewTargetwithBlend (Game|GetPlayerController 0) NewParam 1.5 "VTBlend_Cubic" 1.0 false))

(event Custom|TransitionToLinkedMenu_Event_0
  (params (MenuIndex :type Integer))
  (if (Utilities|Array|IsValidIndex (Variables|Default|GetLinkedMenus) MenuIndex)
    (CallFunction|Transitionto (Utilities|Array|Get(acopy) (Variables|Default|GetLinkedMenus) MenuIndex))))

(event EventBeginPlay
  (bind _aswbp_menu_3d (Utilities|Casting|CastToWBP_Menu3D (UserInterface|GetUserWidgetObject (Variables|Default|GetWidget))))
  (EventDispatchers|AssignTransitiontoLinkedMenu _aswbp_menu_3d (delegate Custom|TransitionToLinkedMenu_Event_0)))

(fn ConstructionScript)