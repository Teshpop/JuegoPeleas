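; BP_ChargeBall is a charged projectile special attack tied to the BP_Combo player character, which it caches on BeginPlay.
; Charge loops on a short delay while the player's Charging flag is set, growing the mesh and damage up to MaxScale and pinning the ball to the player's Arrow2.
; Launch fires it along the player's forward vector through ProjectileMovement, and the actor destroys itself after a fixed lifetime.
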(event EventBeginPlay
  (bind _asbp_combo (Utilities|Casting|CastToBP_Combo (Game|GetPlayerCharacter 0)))
  (Variables|Default|SetPlayer%20Ref _asbp_combo)
  (Utilities|FlowControl|RetriggerableDelay 1e+01)
  (Utilities|IsValid self
    (:Is%20Valid
      (Actor|DestroyActor))))

(event EventCharge
  (bind _staticmesh (Variables|Default|GetStaticMesh))
  (bind _max_scale (Variables|Default|GetMax%20Scale))
  (bind _staticmesh_2 (Variables|Default|GetStaticMesh))
  (bind _relativescale3d (Variables|/Script/Engine.SceneComponent|GetRelativeScale3D _staticmesh))
  (bind (_x _y _z) (Class|KismetMathLibrary|BreakVector3f _relativescale3d))
  (if (Variables|/Game/Felipe/BP_Combo.BP_Combo_C|GetCharging? (Variables|Default|GetPlayer%20Ref)) :!label _label
    (if (Math|Boolean|ANDBoolean (< _x _max_scale) (< _y _max_scale) (< _z _max_scale))
      (Transformation|SetRelativeScale3D _staticmesh_2 (+ (Variables|/Script/Engine.SceneComponent|GetRelativeScale3D _staticmesh_2) "0.005000,0.005000,0.005000"))
      (Variables|Default|SetDamage (+ (Variables|Default|GetDamage) 0.105)))
    (Transformation|SetActorLocation (Transformation|GetWorldLocation (Variables|/Game/Felipe/BP_Combo.BP_Combo_C|GetArrow2 (Variables|Default|GetPlayer%20Ref))) false false)
    (Utilities|FlowControl|RetriggerableDelay 0.01)
    (goto _label)))

(event EventLaunch
  (bind _projectilemovement (Variables|Default|GetProjectileMovement))
  (bind _player_ref (Variables|Default|GetPlayer%20Ref))
  (bind _output_get (Variables|/Script/Engine.ProjectileMovementComponent|SetMaxSpeed _projectilemovement 1e+03))
  (Variables|/Script/Engine.MovementComponent|SetVelocity _projectilemovement (+ (Transformation|GetActorForwardVector _player_ref) (* (Transformation|GetActorForwardVector _player_ref) _output_get))))

(fn ConstructionScript)